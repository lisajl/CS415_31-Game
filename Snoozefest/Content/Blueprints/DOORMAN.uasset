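; DOORMAN is a gatekeeper Blueprint that reacts when the player overlaps its capsule, checking how many collectibles they hold.
; With at least ten, it opens the Question1 widget, shows the mouse cursor and switches to UI-only input.
; Otherwise it briefly shows a dialogue widget, using a DoOnce that resets after removal so repeat overlaps cannot stack it.
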(event `self.CapsuleComponent.OnComponentBeginOverlap`
  (params (OverlappedComponent :type "PrimitiveComponent Object Reference") (OtherActor :type "Actor Object Reference") (OtherComp :type "PrimitiveComponent Object Reference") (OtherBodyIndex :type Integer) (bFromSweep :type Boolean) (SweepResult :type "HitResult Structure (by ref)"))
  (bind _returnvalue (`GameplayStatics.GetPlayerController` 0))
  (bind _asbp_player (cast `/Game/Blueprints/BP_Player` OtherActor))
  (if (>= (`/Game/Blueprints/BP_Player.collectibles` _asbp_player) 10.0)
    (bind _returnvalue_2 (`|CreateWidget` "/Game/Widgets/Question1.Question1_C"))
    (bind _output_get (set `self.q1` _returnvalue_2))
    (`UserWidget.AddToViewport` _output_get 0)
    (set `PlayerController.bShowMouseCursor` true _returnvalue)
    (`WidgetBlueprintLibrary.SetInputMode_UIOnlyEx` _returnvalue _returnvalue_2)
    (else
      (`/Engine/EditorBlueprintResources/StandardMacros.DoOnce` false :!label _label
        (:`Completed`
          (bind _returnvalue_3 (`|CreateWidget` "/Game/Widgets/wb_dialouge.wb_dialouge_C"))
          (bind _output_get_2 (set `self.NewVar` _returnvalue_3))
          (`UserWidget.AddToViewport` _output_get_2 0)
          (`KismetSystemLibrary.Delay` 1.5)
          (`Widget.RemoveFromParent` (`self.NewVar`))
          (goto _label :!via `Reset`))))))

(fn `UserConstructionScript`)