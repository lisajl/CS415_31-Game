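; BP_Mummy is a 2D flipbook enemy character that patrols along the X axis until killed.
; Tick switches idle and walk flipbooks by velocity and drives movement, with a forward line trace triggering a brief pause and reversal, gated by DoOnce.
; Damage reduces health and launches it horizontally away from the causer.
; At zero health it stops updating, plays death flipbooks, removes its capsule and later destroys itself.
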(event `self.ReceiveBeginPlay`
  (set `CharacterMovementComponent.MaxWalkSpeed` (`self.Max Walk Speed`) (`self.CharacterMovement`)))

(event `self.ReceiveTick`
  (params (DeltaSeconds :type "Float (single-precision)"))
  (if (not (`self.MummyDead`))
    (`self.Animation Update`)
    (`self.Movement Update`)))

(event `Animation Update`
  (`PaperFlipbookComponent.SetFlipbook` (`self.Sprite`) (select `bool` (> (`KismetMathLibrary.VSize` (`MovementComponent.Velocity` (`self.CharacterMovement`))) 0.0) :`false` (`self.mummy_idle`) :`true` (`self.mummy_walk`))))

(event `Movement Update`
  (bind _returnvalue (`self.K2_GetActorLocation`))
  ;[1 1 1] Enemy Movement
  (`|ExecutionSequence`
    (:`then_0`
      (if (> (`self.movement_direction`) 0.0)
        (`self.K2_SetActorRotation` (struct))
        (else
          (`self.K2_SetActorRotation` (struct :`Yaw` 180.0)))))
    (:`then_1`
      (`self.AddMovementInput` (1.0 0.0 0.0) (`self.movement_direction`))
      (bind (_outhit _returnvalue_2) (`KismetSystemLibrary.LineTraceSingle` _returnvalue (+ (* (`self.GetActorForwardVector`) (300.0 0.0 0.0)) _returnvalue) "TraceTypeQuery1"))
      (if _returnvalue_2
        (`/Engine/EditorBlueprintResources/StandardMacros.DoOnce` false :!label _label
          (:`Completed`
            (set `CharacterMovementComponent.MaxWalkSpeed` 0.0 (`self.CharacterMovement`))
            (`KismetSystemLibrary.Delay` 0.2)
            (set `CharacterMovementComponent.MaxWalkSpeed` (`self.Max Walk Speed`) (`self.CharacterMovement`))
            (set `self.movement_direction` (* (`self.movement_direction`) -1.0))
            (goto _label :!via `Reset`)))))))

(event `self.ReceiveAnyDamage`
  (params (Damage :type "Float (single-precision)") (DamageType :type "DamageType Object Reference") (InstigatedBy :type "Controller Object Reference") (DamageCauser :type "Actor Object Reference"))
  (bind _returnvalue_x (`KismetMathLibrary.BreakVector` (`KismetMathLibrary.Normal` (`KismetMathLibrary.GetDirectionUnitVector` (`self.K2_GetActorLocation` DamageCauser) (`self.K2_GetActorLocation`)))))
  ;[1 1 1] Damage Done
  (set `self.mummy_health` (- (`self.mummy_health`) Damage))
  (`self.LaunchCharacter` (`KismetMathLibrary.MakeVector` (`KismetMathLibrary.Conv_Int64ToDouble` (* (select `bool` (< _returnvalue_x 0.0) :`false` -1 :`true` 1) -1500))) true true)
  (if (<= (`self.mummy_health`) 0.0)
    (set `self.MummyDead` true)
    (`PaperFlipbookComponent.SetFlipbook` (`self.Sprite`) "/Game/Assets/characters/Mummy/fb_mummy_die.fb_mummy_die")
    (`KismetSystemLibrary.Delay` 0.5)
    (`PaperFlipbookComponent.SetFlipbook` (`self.Sprite`) "/Game/Assets/characters/Mummy/fb_mummy_dead.fb_mummy_dead")
    (`ActorComponent.K2_DestroyComponent` (`self.CapsuleComponent`))
    (`KismetSystemLibrary.Delay` 5.0)
    (`self.K2_DestroyActor`)
    (else
      (set `self.MummyDead` false))))

(fn `UserConstructionScript`)