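; BP_lamp3 is a level exit that opens MainMap3 when a BP_Player with enough collectibles overlaps its capsule.
; On a successful overlap it calls the level load, then resets the player's health and collectible count.
; Otherwise it briefly shows a Wb_dialouge widget, using a DoOnce that resets after removal to prevent stacked popups.
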(event `self.Capsule.OnComponentBeginOverlap`
  (params (OverlappedComponent :type "PrimitiveComponent Object Reference") (OtherActor :type "Actor Object Reference") (OtherComp :type "PrimitiveComponent Object Reference") (OtherBodyIndex :type Integer) (bFromSweep :type Boolean) (SweepResult :type "HitResult Structure (by ref)"))
  (bind _asbp_player (cast `/Game/Blueprints/BP_Player` OtherActor))
  (if (>= (`/Game/Blueprints/BP_Player.collectibles` _asbp_player) 10.0)
    (`GameplayStatics.OpenLevelBySoftObjectPtr` "/Game/Maps/MainMap3.MainMap3")
    (set `/Game/Blueprints/BP_Player.health` 100.0 _asbp_player)
    (set `/Game/Blueprints/BP_Player.collectibles` 0.0 _asbp_player)
    (else
      (`/Engine/EditorBlueprintResources/StandardMacros.DoOnce` false :!label _label
        (:`Completed`
          (bind _returnvalue (`|CreateWidget` "/Game/Widgets/wb_dialouge.wb_dialouge_C"))
          (bind _output_get (set `self.NewVar` _returnvalue))
          (`UserWidget.AddToViewport` _output_get 0)
          (`KismetSystemLibrary.Delay` 1.5)
          (`Widget.RemoveFromParent` (`self.NewVar`))
          (goto _label :!via `Reset`))))))

(fn `UserConstructionScript`)